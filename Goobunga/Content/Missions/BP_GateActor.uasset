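; Mission-driven gate actor that registers with the mission subsystem for open and close tag events.
; Opening plays an FMOD sound and runs a timeline that moves the gate mesh along Z by a configurable offset.
; Closing enables box collision, plays the close sound from a hard-coded position and reverses the same timeline.
; The timeline stops audio on finishing and records its position in milliseconds, though that value feeds only unused logic.
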(event EventBeginPlay
  (bind _returnvalue (Subsystems|GetMissionSubsystem))
  (bind _self self)
  (Class|MissionSubsystem|RegisterforEvent _returnvalue _self (Variables|Default|GetOpenTag))
  (Class|MissionSubsystem|RegisterforEvent _returnvalue _self (Variables|Default|GetCloseTag)))

(event EventTick
  (params (DeltaSeconds :type Float%20%28single-precision%29)))

(event EventEvent
  (params (Tag :type Gameplay%20Tag%20Structure))
  (bind _fmodaudio (Variables|Default|GetFMODAudio))
  (bind _fmodaudio_2 (Variables|Default|GetFMODAudio))
  (|SwitchGameplayTag Tag
    (:Event.OpenGate
      (Class|FMODAudioComponent|SetEvent _fmodaudio_2 (Variables|Default|GetOpenSound))
      (Class|FMODAudioComponent|Play _fmodaudio_2)
      (bind (_direction _open _time) (Timeline|GateOpenTimeline PlayFromStart)
        (:Update
          (Variables|Default|SetCurrentGatePosition (Math|Float|Floor (* _time 1e+03)))
          (Transformation|SetRelativeLocation (Variables|Default|GetGateMesh) (Math|Vector|MakeVector 0.0 0.0 (* _open (Variables|Default|GetGateOffset))) false true))
        (:Finished
          (Class|FMODAudioComponent|Stop (Variables|Default|GetFMODAudio)))))
    (:Event.CloseGate
      (Collision|SetCollisionEnabled (Variables|Default|GetBox) "QueryAndPhysics")
      (Class|FMODAudioComponent|Stop _fmodaudio)
      (Class|FMODAudioComponent|SetEvent _fmodaudio (Variables|Default|GetCloseSound))
      (Class|FMODAudioComponent|Play _fmodaudio)
      (Class|FMODAudioComponent|SetTimelinePosition _fmodaudio 5000)
      (Timeline|GateOpenTimeline Reverse))))

(fn ConstructionScript)