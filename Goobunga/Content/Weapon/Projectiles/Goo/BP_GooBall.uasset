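; BP_GooBall is a short-lived goo projectile that plays a goop sound on spawn and expires after three seconds.
; The construction script randomizes the sphere's scale on each axis for varied blob shapes.
; Any sphere hit simply destroys the ball.
; Disconnected logic that would ragdoll and launch a BP_PepperFiend, or spawn a Niagara burst on other impacts, never runs.
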(event OnComponentHit(Sphere)
  (params (HitComponent :type Primitive%20Component%20Object%20Reference) (OtherActor :type Actor%20Object%20Reference) (OtherComp :type Primitive%20Component%20Object%20Reference) (NormalImpulse :type Vector :default "0, 0, 0") (Hit :type Hit%20Result%20Structure%20%28by%20ref%29))
  (Actor|DestroyActor))

(event EventBeginPlay
  (Audio|PlaySound2D "/Game/Sounds/FX/Weapons/GooGun/SC_GoopSound1.SC_GoopSound1" 1.0 1.0 0.0 0 0)
  (Actor|SetLifeSpan 3.0))

(fn ConstructionScript
  (Transformation|SetWorldScale3D (Variables|Default|GetSphere) (Math|Vector|MakeVector (Math|Random|RandomFloatinRange 0.05 0.1) (Math|Random|RandomFloatinRange 0.05 0.1) (Math|Random|RandomFloatinRange 0.05 0.1))))