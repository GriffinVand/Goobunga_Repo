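; Actor component that plays looping 2D flipbook animations on dynamic material instances by swapping their textures.
; Materials are registered by name, and PlayAnimation gives one a fresh copy of a named entry from the Animations map.
; Each tick, every registered material with an animation accumulates delta time, advances a frame when the frame-rate interval elapses, wraps at the end, and writes that frame to the "Param" texture parameter.
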(event EventTick
  (params (DeltaSeconds :type Float%20%28single-precision%29))
  (CallFunction|UpdateComponent))

(fn AddMaterial
  (params (Material%20Name :type Name) (Dynamic%20Instance :type Material%20Instance%20Dynamic%20Object%20Reference))
  (Utilities|Map|Add (Variables|Default|GetMaterialNameMap) Material%20Name Dynamic%20Instance))

(fn PlayAnimation
  (params (Material%20Name :type Name) (Animation :type Name))
  (bind _materialnamemap (Variables|Default|GetMaterialNameMap))
  (bind _animations (Variables|Default|GetAnimations))
  (bind (_value _returnvalue) (Utilities|Map|Find _materialnamemap Material%20Name))
  (bind (_value_2 _returnvalue_2) (Utilities|Map|Find _animations Animation))
  (bind (_name _frames _framerate) (Utilities|Struct|BreakSTRUCT_2DAnimation _value_2))
  (if (and _returnvalue _returnvalue_2)
    (Utilities|Map|Add (Variables|Default|GetAnimatedMaterials) _value (Utilities|Struct|MakeSTRUCT_2DAnimation _name _frames _framerate))))

(fn UpdateAnimation
  (params (Material%20Instance :type Material%20Instance%20Dynamic%20Object%20Reference))
  (bind _returnvalue (Utilities|Time|GetWorldDeltaSeconds))
  (bind _animatedmaterials (Variables|Default|GetAnimatedMaterials))
  (bind (_value _returnvalue_2) (Utilities|Map|Find _animatedmaterials Material%20Instance))
  (bind (_name _frames _framerate _framebuffer _currentframe) (Utilities|Struct|BreakSTRUCT_2DAnimation _value))
  (bind _returnvalue_3 (+ _framebuffer _returnvalue))
  (if _returnvalue_2
    (LocalVariables|SetCurrentFrame _currentframe)
    (LocalVariables|SetFrameBuffer _returnvalue_3)
    (if (>= _returnvalue_3 (/ 1.0 _framerate))
      (bind _result (Math|Integer|IncrementInt (LocalVariables|GetCurrentFrame))
        (:%20%20
          (LocalVariables|SetFrameBuffer 0.0)
          (if (>= _result (Utilities|Array|Length _frames))
            (LocalVariables|SetCurrentFrame 0)))))
    (Utilities|Map|Add _animatedmaterials Material%20Instance (Utilities|Struct|MakeSTRUCT_2DAnimation _name _frames _framerate (LocalVariables|GetFrameBuffer) (LocalVariables|GetCurrentFrame)))
    (CallFunction|UpdateMaterial Material%20Instance)))

(fn UpdateMaterial
  (params (Material :type Material%20Instance%20Dynamic%20Object%20Reference))
  (bind _animatedmaterials (Variables|Default|GetAnimatedMaterials))
  (bind (_value _returnvalue) (Utilities|Map|Find _animatedmaterials Material))
  (bind (_name _frames _framerate _framebuffer _currentframe) (Utilities|Struct|BreakSTRUCT_2DAnimation _value))
  (if _returnvalue
    (Rendering|Material|SetTextureParameterValue Material "Param" (Utilities|Array|Get(acopy) _frames _currentframe))))

(fn UpdateComponent
  (bind _materialnamemap (Variables|Default|GetMaterialNameMap))
  (bind _keys (Utilities|Map|Keys _materialnamemap))
  (for _array_element _keys
    (CallFunction|UpdateAnimation (.Value (Utilities|Map|Find _materialnamemap _array_element)))))