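; Utility Blueprint that calculates the aim-down-sights offset aligning a weapon's Sight_Socket with the camera.
; The Construction Script stores the skeletal mesh's HipTransform, applies inverted camera-space sight offsets to TestMesh, and saves the resulting ADSTransform.
; FartFunction, uncalled here, tries a quaternion-delta method using the hand_R bone as pivot, printing a forward-vector dot product to check alignment.
; The event graph has no active logic.
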(event EventBeginPlay)

(event Collision|EventActorBeginOverlap
  (params (OtherActor :type Actor%20Object%20Reference)))

(event EventTick
  (params (DeltaSeconds :type Float%20%28single-precision%29)))

(fn ConstructionScript
  (bind _weaponmesh (Variables|Default|GetWeaponMesh))
  (bind _camera (Variables|Default|GetCamera))
  (bind _returnvalue (Transformation|GetWorldTransform _camera))
  (bind _returnvalue_2 (Transformation|GetSocketTransform _weaponmesh "Sight_Socket" "RTS_World"))
  (bind _returnvalue_3 (Math|Transform|InverseTransformRotation _returnvalue (.rotation _returnvalue_2)))
  (Variables|Default|SetHipTransform (Transformation|GetRelativeTransform (Variables|Default|GetSkeletalMesh)))
  (bind _output_get (Variables|Default|SetADSRot (Math|Rotator|MakeRotator (* (.pitch _returnvalue_3) 1.0) (* (.roll _returnvalue_3) 1.0) (* (.yaw _returnvalue_3) -1.0))))
  (Transformation|AddRelativeRotation (Variables|Default|GetTestMesh) _output_get false false)
  (bind _output_get_2 (Variables|Default|SetADSLoc (* (Math|Transform|InverseTransformLocation _returnvalue (.location (Transformation|GetSocketTransform (Variables|Default|GetWeaponMesh1) "Sight_Socket" "RTS_World"))) "-1.000000,-1.000000,-1.000000")))
  (Transformation|AddRelativeLocation (Variables|Default|GetTestMesh) _output_get_2 false false)
  (Variables|Default|SetADSTransform (Transformation|GetRelativeTransform (Variables|Default|GetTestMesh))))

(fn FartFunction
  (bind _weaponmesh (Variables|Default|GetWeaponMesh))
  (bind _weaponmesh_2 (Variables|Default|GetWeaponMesh))
  (bind _camera (Variables|Default|GetCamera))
  (bind _skeletalmesh (Variables|Default|GetSkeletalMesh))
  (bind _weaponmesh_3 (Variables|Default|GetWeaponMesh))
  (bind _skeletalmesh_2 (Variables|Default|GetSkeletalMesh))
  (bind _camera_2 (Variables|Default|GetCamera))
  (bind _returnvalue (Transformation|GetWorldTransform _camera))
  (bind _returnvalue_2 (Transformation|GetWorldTransform _camera_2))
  (bind _returnvalue_3 (Transformation|GetBoneTransform _skeletalmesh "hand_R" "RTS_World"))
  (bind _returnvalue_4 (Transformation|GetSocketTransform _weaponmesh_2 "Sight_Socket" "RTS_World"))
  (bind _returnvalue_5 (Transformation|GetWorldTransform _skeletalmesh_2))
  (bind _returnvalue_6 (Math|Conversions|ToQuaternion(Rotator) (.rotation _returnvalue)))
  (bind _returnvalue_7 (Math|Conversions|ToQuaternion(Rotator) (.rotation _returnvalue_4)))
  (bind _returnvalue_8 (Class|KismetMathLibrary|QuatInversed _returnvalue_7))
  (bind _returnvalue_9 (* _returnvalue_6 _returnvalue_8))
  (Transformation|SetRelativeLocation _weaponmesh "0, 0, 0" false true)
  (Transformation|SetRelativeRotation _weaponmesh "0, 0, 0" false false)
  (Variables|Default|SetADSRot (Math|Transform|InverseTransformRotation _returnvalue_5 (Class|KismetMathLibrary|QuatRotator _returnvalue_9)))
  (Transformation|SetWorldRotation _weaponmesh_3 (Transformation|GetWorldRotation (Variables|Default|GetWeaponMesh)) false false)
  (Transformation|AddWorldRotation _weaponmesh_3 (Variables|Default|GetADSRot) false false)
  (Development|PrintString (Utilities|String|ToString(Float) (Math|Vector|DotProduct (Math|Vector|GetForwardVector (Transformation|GetSocketRotation _weaponmesh_3 "Sight_Socket")) (Math|Vector|GetForwardVector (.rotation _returnvalue_2)))))
  (Variables|Default|SetADSLoc (Math|Transform|InverseTransformLocation _returnvalue_5 (- (.location _returnvalue_2) (- (+ (.location _returnvalue_3) (Class|KismetMathLibrary|QuatRotateVector _returnvalue_9 (- (.location (Transformation|GetSocketTransform (Variables|Default|GetWeaponMesh) "Sight_Socket" "RTS_World")) (.location _returnvalue_3)))) (.location _returnvalue_3))))))