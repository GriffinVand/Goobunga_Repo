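; Evil wizard interactable that offers a pepper to buy and launches the intro mission.
; It is always interactable; interacting plays munch and hurt sounds, hides the pepper mesh and disables interaction collision.
; It then ends the player's interaction, selects the intro mission on the game instance and has the player fade and load Level 1.
; No cost or currency check runs despite the "Buy Pepper" prompt.
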(event EventBeginPlay)

(event Collision|EventActorBeginOverlap
  (params (OtherActor :type Actor%20Object%20Reference)))

(event EventTick
  (params (DeltaSeconds :type Float%20%28single-precision%29)))

(event EventInteract
  (params (Interactor :type Actor%20Object%20Reference))
  (Class|FMODBlueprintStatics|PlayEvent2D "/Game/FMOD/Events/FXEvents/BananaMunch.BananaMunch")
  (Class|FMODBlueprintStatics|PlayEvent2D "/Game/FMOD/Events/FXEvents/PlayerHurt.PlayerHurt")
  (Rendering|SetVisibility (Variables|Default|GetPepperMesh) false false)
  (Collision|SetCollisionEnabled (Variables|Default|GetInteractCollision) "NoCollision")
  (bind _asgoobunga_player (Utilities|Casting|CastToGoobunga_Player Interactor))
  (Class|PlayerCallables|EndInteract _asgoobunga_player self)
  (bind _asbp_goobunga_game_instance (Utilities|Casting|CastToBP_GoobungaGameInstance (Game|GetGameInstance)))
  (Class|GoobungaGameInstance|SelectMission _asbp_goobunga_game_instance "/Game/Missions/MissionData/DA_IntroMission.DA_IntroMission")
  (Class|GoobungaPlayer|FadeandLoad _asgoobunga_player "L_Level1"))

(fn ConstructionScript)

(fn GetInteractText
  (params (Interactor :type Actor%20Object%20Reference))
  (return "Press 'E' Buy Pepper"))

(fn CanInteract
  (return true))