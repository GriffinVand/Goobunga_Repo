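; Player character Blueprint for Goobunga, with a first-person mesh, an equipped cat gun and facial animation.
; On BeginPlay it spawns BP_CatGun as the equipped item, snaps it to the mesh's cat socket, sets itself as owner, and adds crosshair and temporary face-cam widgets.
; The construction script creates a dynamic Griffin face material, hands it to FacialAnimationComponent and applies it to the first-person mesh.
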(event EventBeginPlay
  (bind _returnvalue (Game|SpawnActorfromClass "/Game/Weapon/Weapons/CatGun/BP_CatGun.BP_CatGun_C" (Math|Transform|MakeTransform "0, 0, 0" "0, 0, 0" "1.000000,1.000000,1.000000") "Undefined" "MultiplyWithRoot" 0 0))
  (bind _output_get (Variables|Default|SetEquippedItem _returnvalue))
  (Transformation|AttachComponentToComponent _output_get (Variables|Default|GetFPMesh) "Cat_Socket" "SnapToTarget" "SnapToTarget" "SnapToTarget" true)
  (Variables|/Script/Goobunga.Weapon|SetWeaponOwner _returnvalue self)
  (bind _returnvalue_2 (UserInterface|CreateWidget "/Game/UI/WBP_Crosshair.WBP_Crosshair_C"))
  (UserInterface|Viewport|AddtoViewport _returnvalue_2 0)
  (bind _returnvalue_3 (UserInterface|CreateWidget "/Game/UI/FaceCam/WBP_FaceCam_Temp.WBP_FaceCam_Temp_C"))
  (UserInterface|Viewport|AddtoViewport _returnvalue_3 0))

(fn ConstructionScript
  (bind _returnvalue (Rendering|Material|CreateDynamicMaterialInstance "/Game/Characters/Player/Materials/MI_Griffin_Face.MI_Griffin_Face" "None" "None" :!class /Script/Engine.KismetMaterialLibrary))
  (bind _output_get (Variables|/Script/Goobunga.FacialAnimationComponent|SetMaterial (Variables|Default|GetFacialAnimationComponent) _returnvalue))
  (Rendering|Material|SetMaterial (Variables|Default|GetFPMesh) 1 _output_get))