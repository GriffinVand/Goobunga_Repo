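; Test actor for Pepper Fiend dismemberment that bursts a set of body-part meshes apart with physics.
; The construction script creates a mesh component for each listed static mesh, ignoring Pawn collision and storing it in an array.
; Shortly after BeginPlay, each component starts simulating physics and receives a radial impulse from the scene root.
; A trailing delayed loop over the components has an empty body.
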(event EventBeginPlay
  (Utilities|FlowControl|Delay 2.0)
  (for _array_element (Variables|Default|GetStaticMeshInstances)
    (Physics|SetSimulatePhysics _array_element true)
    (Physics|AddRadialImpulse _array_element (Transformation|GetWorldLocation (Variables|Default|GetDefaultSceneRoot)) 1e+03 1e+03 "RIF_Constant" false)
    (Utilities|FlowControl|Delay 1.0)
    (for _array_element_2 (Variables|Default|GetStaticMeshInstances)
      _)))

(fn ConstructionScript
  (for _array_element (Variables|Default|GetStaticMeshes)
    (bind _returnvalue (AddComponent|AddStaticMeshComponent false))
    (Components|StaticMesh|SetStaticMesh _returnvalue _array_element)
    (Collision|SetCollisionResponsetoChannel _returnvalue "ECC_Pawn" "ECR_Ignore")
    (Utilities|Array|Add (Variables|Default|GetStaticMeshInstances) _returnvalue)))