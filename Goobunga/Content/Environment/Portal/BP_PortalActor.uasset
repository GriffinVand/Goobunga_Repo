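; BP_PortalActor is a portal actor that stays transparent until a mission event makes it visible.
; On BeginPlay it creates a dynamic material instance for the Portal component, sets PortalOpacity to zero and registers with the MissionSubsystem for the Event.Special2 tag.
; Its Event handler sets PortalOpacity to one, switching the portal on instantly with no fade.
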(event EventBeginPlay
  (bind _portal (Variables|Default|GetPortal))
  (bind _returnvalue (Rendering|Material|CreateDynamicMaterialInstance (Rendering|Material|GetMaterial _portal 0) "None" "None" :!class /Script/Engine.KismetMaterialLibrary))
  (bind _output_get (Variables|Default|SetPortaMat _returnvalue))
  (Rendering|Material|SetScalarParameterValue _output_get "PortalOpacity" 0.0 :!class /Script/Engine.MaterialInstanceDynamic)
  (Rendering|Material|SetMaterial _portal 0 _output_get)
  (Class|MissionSubsystem|RegisterforEvent (Subsystems|GetMissionSubsystem) self "(TagName=\"Event.Special2\")"))

(event EventEvent
  (params (Tag :type Gameplay%20Tag%20Structure))
  (Rendering|Material|SetScalarParameterValue (Variables|Default|GetPortaMat) "PortalOpacity" 1.0 :!class /Script/Engine.MaterialInstanceDynamic))

(fn ConstructionScript)