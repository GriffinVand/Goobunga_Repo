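; Goo gun projectile that leaves a slime splat on whatever it hits, ignoring the first player's pawn.
; Construction gives the sphere a random small scale on each axis, so each blob differs in shape.
; On spawn it plays a goop sound and sets a short lifespan.
; On hit it spawns a fading slime decal oriented from actor to impact point, adds a Niagara burst and destroys itself.
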(event OnComponentHit(Sphere)
  (params (HitComponent :type Primitive%20Component%20Object%20Reference) (OtherActor :type Actor%20Object%20Reference) (OtherComp :type Primitive%20Component%20Object%20Reference) (NormalImpulse :type Vector :default "0, 0, 0") (Hit :type Hit%20Result%20Structure%20%28by%20ref%29))
  (bind _returnvalue (Transformation|GetActorLocation))
  (bind _impactpoint (Collision|BreakHitResult Hit))
  (bind _returnvalue_2 (Math|Rotator|FindLookatRotation _returnvalue _impactpoint))
  (if (!= OtherActor (Game|Player|GetPlayerPawn 0))
    (bind _returnvalue_3 (Rendering|Decal|SpawnDecalatLocation "/Game/Weapons/GooGun/GooGunProjectile/Slime_Mat.Slime_Mat" "100.000000,100.000000,100.000000" _impactpoint (Math|Rotator|MakeRotator (.roll _returnvalue_2) (.pitch _returnvalue_2) (.yaw _returnvalue_2)) 0.0))
    (Rendering|Components|Decal|SetFadeOut _returnvalue_3 0.0 4.0 true)
    (Niagara|SpawnSystematLocation "/Game/Effects/NS_Burst.NS_Burst" _impactpoint)
    (Actor|DestroyActor)))

(event EventBeginPlay
  (Audio|PlaySound2D "/Game/Sounds/Weapons/GooGun/SC_GoopSound1.SC_GoopSound1" 1.0 1.0 0.0 0 0)
  (Actor|SetLifeSpan 3.0))

(fn ConstructionScript
  (Transformation|SetWorldScale3D (Variables|Default|GetSphere) (Math|Vector|MakeVector (Math|Random|RandomFloatinRange 0.05 0.1) (Math|Random|RandomFloatinRange 0.05 0.1) (Math|Random|RandomFloatinRange 0.05 0.1))))